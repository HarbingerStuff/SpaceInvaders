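; BP_Enemy is a Space Invaders-style formation of 14 cube enemies in one actor that marches and shoots.
; BeginPlay loops latent Left, Down, Right, Down moves on the root, alongside a half-second delay loop picking a random cube to fire BP_EnemyProjectile if still valid.
; Each cube has a Hit macro instance serving both firing and box overlaps, where a BP_ShipProjectile destroys cube, box and itself, incrementing EnemyHit.
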(event `self.ReceiveBeginPlay`
  (bind _cube3 (`self.Cube3`))
  (bind _cube4 (`self.Cube4`))
  (bind _cube5 (`self.Cube5`))
  (bind _cube6 (`self.Cube6`))
  (bind _cube7 (`self.Cube7`))
  (bind _cube (`self.Cube`))
  (bind _cube8 (`self.Cube8`))
  (bind _cube9 (`self.Cube9`))
  (bind _cube10 (`self.Cube10`))
  (bind _cube11 (`self.Cube11`))
  (bind _cube12 (`self.Cube12`))
  (bind _cube13 (`self.Cube13`))
  (bind _cube1 (`self.Cube1`))
  (bind _cube2 (`self.Cube2`))
  (`|ExecutionSequence`
    (:`then_0`
      (`self.Left` :!label _label
        (:`Completed`
          (`self.Down`
            (:`Completed`
              (`self.Right`
                (:`Completed`
                  (`self.Down`
                    (:`Completed`
                      (goto _label))))))))))
    (:`then_1`
      (bind _output_get (set `self.RandomInt` (`KismetMathLibrary.RandomIntegerInRange` 0 13) :!label _label_2))
      (`KismetSystemLibrary.RetriggerableDelay` 0.5)
      (`|ExecutionSequence`
        (:`then_0`
          (goto _label_2))
        (:`then_1`
          (switch `int` _output_get
            (:`0`
              (goto _label_3 :!via `Spawn`))
            (:`1`
              (goto _label_4 :!via `Spawn`))
            (:`2`
              (goto _label_5 :!via `Spawn`))
            (:`3`
              (goto _label_6 :!via `Spawn`))
            (:`4`
              (goto _label_7 :!via `Spawn`))
            (:`5`
              (goto _label_8 :!via `Spawn`))
            (:`6`
              (goto _label_9 :!via `Spawn`))
            (:`7`
              (goto _label_10 :!via `Spawn`))
            (:`8`
              (goto _label_11 :!via `Spawn`))
            (:`9`
              (goto _label_12 :!via `Spawn`))
            (:`10`
              (goto _label_13 :!via `Spawn`))
            (:`11`
              (goto _label_14 :!via `Spawn`))
            (:`12`
              (goto _label_15 :!via `Spawn`))
            (:`13`
              (goto _label_16 :!via `Spawn`))))))))

(event `self.Box.OnComponentBeginOverlap`
  (params (OverlappedComponent :type "PrimitiveComponent Object Reference") (OtherActor :type "Actor Object Reference") (OtherComp :type "PrimitiveComponent Object Reference") (OtherBodyIndex :type Integer) (bFromSweep :type Boolean) (SweepResult :type "HitResult Structure (by ref)"))
  (bind _cube (`self.Cube`))
  (`self.Hit` OtherActor _cube (`self.Box`) _cube :!label _label_3))

(event `self.Box1.OnComponentBeginOverlap`
  (params (OverlappedComponent :type "PrimitiveComponent Object Reference") (OtherActor :type "Actor Object Reference") (OtherComp :type "PrimitiveComponent Object Reference") (OtherBodyIndex :type Integer) (bFromSweep :type Boolean) (SweepResult :type "HitResult Structure (by ref)"))
  (bind _cube1 (`self.Cube1`))
  (`self.Hit` OtherActor _cube1 (`self.Box1`) _cube1 :!label _label_4))

(event `self.Box2.OnComponentBeginOverlap`
  (params (OverlappedComponent :type "PrimitiveComponent Object Reference") (OtherActor :type "Actor Object Reference") (OtherComp :type "PrimitiveComponent Object Reference") (OtherBodyIndex :type Integer) (bFromSweep :type Boolean) (SweepResult :type "HitResult Structure (by ref)"))
  (bind _cube2 (`self.Cube2`))
  (`self.Hit` OtherActor _cube2 (`self.Box2`) _cube2 :!label _label_5))

(event `self.Box3.OnComponentBeginOverlap`
  (params (OverlappedComponent :type "PrimitiveComponent Object Reference") (OtherActor :type "Actor Object Reference") (OtherComp :type "PrimitiveComponent Object Reference") (OtherBodyIndex :type Integer) (bFromSweep :type Boolean) (SweepResult :type "HitResult Structure (by ref)"))
  (bind _cube3 (`self.Cube3`))
  (`self.Hit` OtherActor _cube3 (`self.Box3`) _cube3 :!label _label_6))

(event `self.Box4.OnComponentBeginOverlap`
  (params (OverlappedComponent :type "PrimitiveComponent Object Reference") (OtherActor :type "Actor Object Reference") (OtherComp :type "PrimitiveComponent Object Reference") (OtherBodyIndex :type Integer) (bFromSweep :type Boolean) (SweepResult :type "HitResult Structure (by ref)"))
  (bind _cube4 (`self.Cube4`))
  (`self.Hit` OtherActor _cube4 (`self.Box4`) _cube4 :!label _label_7))

(event `self.Box5.OnComponentBeginOverlap`
  (params (OverlappedComponent :type "PrimitiveComponent Object Reference") (OtherActor :type "Actor Object Reference") (OtherComp :type "PrimitiveComponent Object Reference") (OtherBodyIndex :type Integer) (bFromSweep :type Boolean) (SweepResult :type "HitResult Structure (by ref)"))
  (bind _cube5 (`self.Cube5`))
  (`self.Hit` OtherActor _cube5 (`self.Box5`) _cube5 :!label _label_8))

(event `self.Box6.OnComponentBeginOverlap`
  (params (OverlappedComponent :type "PrimitiveComponent Object Reference") (OtherActor :type "Actor Object Reference") (OtherComp :type "PrimitiveComponent Object Reference") (OtherBodyIndex :type Integer) (bFromSweep :type Boolean) (SweepResult :type "HitResult Structure (by ref)"))
  (bind _cube6 (`self.Cube6`))
  (`self.Hit` OtherActor _cube6 (`self.Box6`) _cube6 :!label _label_9))

(event `self.Box7.OnComponentBeginOverlap`
  (params (OverlappedComponent :type "PrimitiveComponent Object Reference") (OtherActor :type "Actor Object Reference") (OtherComp :type "PrimitiveComponent Object Reference") (OtherBodyIndex :type Integer) (bFromSweep :type Boolean) (SweepResult :type "HitResult Structure (by ref)"))
  (bind _cube7 (`self.Cube7`))
  (`self.Hit` OtherActor _cube7 (`self.Box7`) _cube7 :!label _label_10))

(event `self.Box8.OnComponentBeginOverlap`
  (params (OverlappedComponent :type "PrimitiveComponent Object Reference") (OtherActor :type "Actor Object Reference") (OtherComp :type "PrimitiveComponent Object Reference") (OtherBodyIndex :type Integer) (bFromSweep :type Boolean) (SweepResult :type "HitResult Structure (by ref)"))
  (bind _cube8 (`self.Cube8`))
  (`self.Hit` OtherActor _cube8 (`self.Box8`) _cube8 :!label _label_11))

(event `self.Box9.OnComponentBeginOverlap`
  (params (OverlappedComponent :type "PrimitiveComponent Object Reference") (OtherActor :type "Actor Object Reference") (OtherComp :type "PrimitiveComponent Object Reference") (OtherBodyIndex :type Integer) (bFromSweep :type Boolean) (SweepResult :type "HitResult Structure (by ref)"))
  (bind _cube9 (`self.Cube9`))
  (`self.Hit` OtherActor _cube9 (`self.Box9`) _cube9 :!label _label_12))

(event `self.Box10.OnComponentBeginOverlap`
  (params (OverlappedComponent :type "PrimitiveComponent Object Reference") (OtherActor :type "Actor Object Reference") (OtherComp :type "PrimitiveComponent Object Reference") (OtherBodyIndex :type Integer) (bFromSweep :type Boolean) (SweepResult :type "HitResult Structure (by ref)"))
  (bind _cube10 (`self.Cube10`))
  (`self.Hit` OtherActor _cube10 (`self.Box10`) _cube10 :!label _label_13))

(event `self.Box11.OnComponentBeginOverlap`
  (params (OverlappedComponent :type "PrimitiveComponent Object Reference") (OtherActor :type "Actor Object Reference") (OtherComp :type "PrimitiveComponent Object Reference") (OtherBodyIndex :type Integer) (bFromSweep :type Boolean) (SweepResult :type "HitResult Structure (by ref)"))
  (bind _cube11 (`self.Cube11`))
  (`self.Hit` OtherActor _cube11 (`self.Box11`) _cube11 :!label _label_14))

(event `self.Box12.OnComponentBeginOverlap`
  (params (OverlappedComponent :type "PrimitiveComponent Object Reference") (OtherActor :type "Actor Object Reference") (OtherComp :type "PrimitiveComponent Object Reference") (OtherBodyIndex :type Integer) (bFromSweep :type Boolean) (SweepResult :type "HitResult Structure (by ref)"))
  (bind _cube12 (`self.Cube12`))
  (`self.Hit` OtherActor _cube12 (`self.Box12`) _cube12 :!label _label_15))

(event `self.Box13.OnComponentBeginOverlap`
  (params (OverlappedComponent :type "PrimitiveComponent Object Reference") (OtherActor :type "Actor Object Reference") (OtherComp :type "PrimitiveComponent Object Reference") (OtherBodyIndex :type Integer) (bFromSweep :type Boolean) (SweepResult :type "HitResult Structure (by ref)"))
  (bind _cube13 (`self.Cube13`))
  (`self.Hit` OtherActor _cube13 (`self.Box13`) _cube13 :!label _label_16))

(fn `UserConstructionScript`)